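; BP_PendulumTrap is a swinging hazard that knocks the first-person player away and then deals massive damage.
; A looping timeline ping-pongs between play and reverse, lerping the pendulum mesh's relative rotation back and forth.
; Overlapping its sphere launches the player away from the sphere's center with added upward lift, then applies the damage after a short delay.
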(event `self.ReceiveBeginPlay`
  ;[1 1 1] Pendulum Movement
  (bind (_direction _movement) (`Timeline|Movement Timeline` :!label _label)
    (:`Update`
      (`SceneComponent.K2_SetRelativeRotation` (`self.SM_Pendulum`) (`KismetMathLibrary.RLerp` (struct :`Roll` -60.0) (struct :`Roll` 60.0) _movement) false false))
    (:`Finished`
      (if (`|EnumEquality` _direction "Forward")
        (goto _label :!via `Reverse`)
        (else
          (goto _label))))))

(event `self.Sphere.OnComponentBeginOverlap`
  (params (OverlappedComponent :type "PrimitiveComponent Object Reference") (OtherActor :type "Actor Object Reference") (OtherComp :type "PrimitiveComponent Object Reference") (OtherBodyIndex :type Integer) (bFromSweep :type Boolean) (SweepResult :type "HitResult Structure (by ref)"))
  ;[1 1 1] Pendulum Hit and Launch Player
  (bind _asbp_first_person_character (cast `/Game/FirstPerson/Blueprints/BP_FirstPersonCharacter` OtherActor))
  (bind _output_get (set `self.Overlapped Player` _asbp_first_person_character))
  (`Character.LaunchCharacter` (`self.Overlapped Player`) (+ (* (`KismetMathLibrary.Normal` (- (`SceneComponent.K2_GetComponentLocation` (`self.Sphere`)) (`self.K2_GetActorLocation` _output_get))) -3000.0) (* (`self.GetActorUpVector` (`self.Overlapped Player`)) 800.0)) false false)
  (`KismetSystemLibrary.Delay` 0.5)
  (`GameplayStatics.ApplyDamage` (`self.Overlapped Player`) 40000.0 null self))

(fn `UserConstructionScript`)