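; BP_DoorButton is an interactable button that triggers a referenced door when E is pressed.
; Sphere overlap enables player 0's input, and ending the overlap also calls EnableInput, so input is never disabled.
; On press, the Cylinder eases to Sphere1's relative location, MoveDoor is called on DoorRef, then the Cylinder eases back to the transform cached at BeginPlay.
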(event `self.Sphere.OnComponentBeginOverlap`
  (params (OverlappedComponent :type "PrimitiveComponent Object Reference") (OtherActor :type "Actor Object Reference") (OtherComp :type "PrimitiveComponent Object Reference") (OtherBodyIndex :type Integer) (bFromSweep :type Boolean) (SweepResult :type "HitResult Structure (by ref)"))
  (`self.EnableInput` (`GameplayStatics.GetPlayerController` 0)))

(event `self.ReceiveBeginPlay`
  (bind _cylinder (`self.Cylinder`))
  (set `self.OriginalPos` (`SceneComponent.RelativeLocation` _cylinder))
  (set `self.OriginalRot` (`SceneComponent.RelativeRotation` _cylinder)))

(event `self.Sphere.OnComponentEndOverlap`
  (params (OverlappedComponent :type "PrimitiveComponent Object Reference") (OtherActor :type "Actor Object Reference") (OtherComp :type "PrimitiveComponent Object Reference") (OtherBodyIndex :type Integer))
  (`self.EnableInput` (`GameplayStatics.GetPlayerController` 0)))

(event `Key|E`
  (params (Key :type "Key Structure"))
  (:`Pressed`
    (`KismetSystemLibrary.MoveComponentTo` (`self.Cylinder`) (`SceneComponent.RelativeLocation` (`self.Sphere1`)) (`self.OriginalRot`) true false 0.6)
    (`/Game/Quake/Blueprints/Environment/BP_Door.MoveDoor` (`self.DoorRef`))
    (`KismetSystemLibrary.MoveComponentTo` (`self.Cylinder`) (`self.OriginalPos`) (`self.OriginalRot`) true false 1.0)))

(fn `UserConstructionScript`)