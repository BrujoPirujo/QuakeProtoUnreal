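; A regeneration pickup that heals an overlapping BP_FirstPersonCharacter over time, then respawns after a cooldown.
; On authority, a looping timer calls Regen to heal the stored player until RegenerationTime clears the Healing flag.
; Authority and remote both hide the pickup and disable its sphere until Enable restores them, though remote skips the character check.
; The final PauseTimer names TakePlayerDamage, so the Regen timer keeps ticking, gated only by Healing.
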(event `self.Sphere.OnComponentBeginOverlap`
  (params (OverlappedComponent :type "PrimitiveComponent Object Reference") (OtherActor :type "Actor Object Reference") (OtherComp :type "PrimitiveComponent Object Reference") (OtherBodyIndex :type Integer) (bFromSweep :type Boolean) (SweepResult :type "HitResult Structure (by ref)"))
  (`/Engine/EditorBlueprintResources/ActorMacros.Switch Has Authority`
    (:`Authority`
      (bind _asbp_first_person_character (cast `/Game/FirstPerson/Blueprints/BP_FirstPersonCharacter` OtherActor))
      (set `self.Player` _asbp_first_person_character)
      (set `self.Healing` true)
      (`KismetSystemLibrary.K2_SetTimer` null "Regen" 0.1 true)
      (`|ExecutionSequence`
        (:`then_0`
          (`self.SetActorHiddenInGame` true :!label _label)
          (`PrimitiveComponent.SetCollisionEnabled` (`self.Sphere`) "NoCollision")
          (`KismetSystemLibrary.K2_SetTimerDelegate` (delegate `Enable`) (`self.Time Cooldown`)))
        (:`then_1`
          (`KismetSystemLibrary.Delay` (`self.RegenerationTime`))
          (set `self.Healing` false)
          (`KismetSystemLibrary.K2_PauseTimer` null "TakePlayerDamage"))))
    (:`Remote`
      (goto _label))))

(event `Enable`
  (`self.SetActorHiddenInGame` false)
  (`PrimitiveComponent.SetCollisionEnabled` (`self.Sphere`) "QueryOnly"))

(fn `Regen`
  (if (`self.Healing`)
    (`/Game/FirstPerson/Blueprints/BP_FirstPersonCharacter.Heal Player` (`self.Player`) (`self.HealValue`))))

(fn `UserConstructionScript`)