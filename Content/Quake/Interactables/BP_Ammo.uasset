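; BP_Ammo is a respawning ammo pickup for the first-person character.
; Overlapping its sphere passes the configured ammo amount and weapon to the character's ChangeAmmo, then hides the actor and disables sphere collision.
; A one-shot timer restores visibility and query-only collision after the cooldown, so the same actor is reused instead of destroyed.
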(event `self.Sphere.OnComponentBeginOverlap`
  (params (OverlappedComponent :type "PrimitiveComponent Object Reference") (OtherActor :type "Actor Object Reference") (OtherComp :type "PrimitiveComponent Object Reference") (OtherBodyIndex :type Integer) (bFromSweep :type Boolean) (SweepResult :type "HitResult Structure (by ref)"))
  (bind _asbp_first_person_character (cast `/Game/FirstPerson/Blueprints/BP_FirstPersonCharacter` OtherActor))
  (`/Game/FirstPerson/Blueprints/BP_FirstPersonCharacter.Change Ammo` _asbp_first_person_character (`self.Ammo`) (`self.Weapon`))
  (`self.SetActorHiddenInGame` true)
  (`PrimitiveComponent.SetCollisionEnabled` (`self.Sphere`) "NoCollision")
  (`KismetSystemLibrary.K2_SetTimerDelegate` (delegate `Enable`) (`self.Time Cooldown`)))

(event `Enable`
  (`self.SetActorHiddenInGame` false)
  (`PrimitiveComponent.SetCollisionEnabled` (`self.Sphere`) "QueryOnly"))

(fn `UserConstructionScript`)