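; Player controller that spawns, possesses and despawns the first-person character.
; PlayerStarts are cached at BeginPlay, and the + key triggers Spawn while not spawned.
; Spawn destroys the current pawn and loops sphere overlaps for a clear random start, though the spawn transform comes from a separate random pick.
; Despawn, on authority, swaps the pawn for an empty one; RespawnPlayer is marked unused.
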(event `Key|+`
  (params (Key :type "Key Structure"))
  ;[1 1 1] Press + to spawn
  (:`Pressed`
    (if (not (`self.Spawned`))
      (`self.Spawn`)
      (set `self.Spawned` true))))

(event `SetUp Camera`
  (params (Camera :type "CameraActor Object Reference"))
  (bind _output_get (set `self.Camera ` Camera))
  (`self.SetViewTargetWithBlend` _output_get))

(event `self.ReceiveBeginPlay`
  ;[1 1 1] Gets the Spawn Points at start
  (bind _outactors (`GameplayStatics.GetAllActorsOfClass` "/Script/Engine.PlayerStart"))
  (set `self.Player Start` _outactors))

(event `Respawn Player`
  ;[1 1 1] Respawn at 000, not in use
  (bind _returnvalue (`|SpawnActorFromClass` "/Game/FirstPerson/Blueprints/BP_FirstPersonCharacter.BP_FirstPersonCharacter_C" (`self.Spawn Transform`) "Undefined" "MultiplyWithRoot" null null))
  (`self.Possess` _returnvalue))

(event `Spawn`
  (bind _returnvalue (`self.K2_GetPawn`))
  (bind _player_start (`self.Player Start`))
  (bind _output (`|GetArrayItem` _player_start (`KismetMathLibrary.RandomInteger` (`KismetArrayLibrary.Array_Length` _player_start))))
  ;[1 1 1] Spawn Player at a random spawnpoint
  (`/Engine/EditorBlueprintResources/StandardMacros.IsValid` _returnvalue
    (:`Is Valid`
      (`self.K2_DestroyActor` _returnvalue)
      (while (stale _returnvalue_2)
        (bind (_outactors _returnvalue_2) (`KismetSystemLibrary.SphereOverlapActors` (`self.K2_GetActorLocation` _output) 500.0 (`|MakeArray` "ObjectTypeQuery3" :!type "EObjectTypeQuery Enum") "/Game/FirstPerson/Blueprints/BP_FirstPersonCharacter.BP_FirstPersonCharacter_C")))
      (bind _returnvalue_3 (`|SpawnActorFromClass` "/Game/FirstPerson/Blueprints/BP_FirstPersonCharacter.BP_FirstPersonCharacter_C" (`self.GetTransform` _output) "Undefined" "MultiplyWithRoot" null null))
      (`self.Possess` _returnvalue_3))))

(event `Despawn`
  (bind _returnvalue (`self.K2_GetPawn`))
  ;[1 1 1] Despawns Player and creates an Empty pawn
  (`/Engine/EditorBlueprintResources/StandardMacros.IsValid` _returnvalue
    (:`Is Valid`
      (`/Engine/EditorBlueprintResources/ActorMacros.Switch Has Authority`
        (:`Authority`
          (`self.K2_DestroyActor` _returnvalue)
          (bind _returnvalue_2 (`|SpawnActorFromClass` "/Game/Quake/BluePrints/BP_EmptyPawn.BP_EmptyPawn_C" (`self.GetTransform`) "Undefined" "MultiplyWithRoot" null null))
          (`self.Possess` _returnvalue_2)
          (set `self.Spawned` false))))))

(fn `UserConstructionScript`)