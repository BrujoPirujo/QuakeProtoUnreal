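; BP_Door is a sliding door in the Quake game that opens on a MoveDoor call and returns automatically.
; BeginPlay caches the Door component's starting transform, then MoveDoor eases it to the TargetPos component's location, pauses, and eases it back, keeping the original rotation.
; The DoorClosed flag acts as a busy guard during the cycle, ignoring repeat calls until the door has returned.
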(event `self.ReceiveBeginPlay`
  (bind _door (`self.Door`))
  (set `self.OriginalPos` (`SceneComponent.RelativeLocation` _door))
  (set `self.OriginalRot` (`SceneComponent.RelativeRotation` _door)))

(event `MoveDoor`
  (if (not (`self.DoorClosed`))
    (set `self.DoorClosed` true)
    (`KismetSystemLibrary.MoveComponentTo` (`self.Door`) (`SceneComponent.RelativeLocation` (`self.TargetPos`)) (`self.OriginalRot`) true true 1.0)
    (`KismetSystemLibrary.Delay` 5.0)
    (`KismetSystemLibrary.MoveComponentTo` (`self.Door`) (`self.OriginalPos`) (`self.OriginalRot`) true true 1.0)
    (set `self.DoorClosed` false)))

(fn `UserConstructionScript`)