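; BP_Fire is a fire hazard that repeatedly damages the first-person player character within its sphere trigger.
; Overlap begin stores the character, sets a Burning flag and starts a fast looping timer that calls TakePlayerDamage to apply FireDamage.
; Overlap end waits a short delay before clearing the flag and pausing the timer, so the burn briefly lingers after leaving.
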(event `self.Sphere.OnComponentBeginOverlap`
  (params (OverlappedComponent :type "PrimitiveComponent Object Reference") (OtherActor :type "Actor Object Reference") (OtherComp :type "PrimitiveComponent Object Reference") (OtherBodyIndex :type Integer) (bFromSweep :type Boolean) (SweepResult :type "HitResult Structure (by ref)"))
  (bind _asbp_first_person_character (cast `/Game/FirstPerson/Blueprints/BP_FirstPersonCharacter` OtherActor))
  (set `self.Player` _asbp_first_person_character)
  (set `self.Burning` true)
  (`KismetSystemLibrary.K2_SetTimer` null "TakePlayerDamage" 0.1 true))

(event `self.Sphere.OnComponentEndOverlap`
  (params (OverlappedComponent :type "PrimitiveComponent Object Reference") (OtherActor :type "Actor Object Reference") (OtherComp :type "PrimitiveComponent Object Reference") (OtherBodyIndex :type Integer))
  (cast `/Game/FirstPerson/Blueprints/BP_FirstPersonCharacter` OtherActor)
  (`KismetSystemLibrary.Delay` 0.6)
  (set `self.Burning` false)
  (`KismetSystemLibrary.K2_PauseTimer` null "TakePlayerDamage"))

(fn `TakePlayerDamage`
  (if (`self.Burning`)
    (`GameplayStatics.ApplyDamage` (`self.Player`) (`self.Fire_Damage`) null self)))

(fn `UserConstructionScript`)