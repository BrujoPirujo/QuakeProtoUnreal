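; First-person player controller for the Quake game that handles spawning, possession, despawning and kill/death counts.
; The + key spawns and possesses a BP_FirstPersonCharacter at a PlayerStart gathered on BeginPlay.
; A sphere-overlap loop tests for nearby characters, but its random spawn lookup is separate from the one used for spawning.
; Despawn swaps in an empty pawn to allow respawning, and holding Tab shows the character's K/D widget.
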(event `Key|+`
  (params (Key :type "Key Structure"))
  ;[1 1 1] Press + to spawn
  (:`Pressed`
    (if (not (`self.Spawned`))
      (`self.Spawn`)
      (set `self.Spawned` true))))

(event `SetUp Camera`
  (params (Camera :type "CameraActor Object Reference"))
  ;[1 1 1] SetUp Camera
  (bind _output_get (set `self.Camera ` Camera))
  (`self.SetViewTargetWithBlend` _output_get))

(event `self.ReceiveBeginPlay`
  ;[1 1 1] Gets the Spawn Points at start
  (bind _outactors (`GameplayStatics.GetAllActorsOfClass` "/Script/Engine.PlayerStart"))
  (set `self.Player Start` _outactors))

(event `Spawn`
  (bind _returnvalue (`self.K2_GetPawn`))
  (bind _player_start (`self.Player Start`))
  (bind _output (`|GetArrayItem` _player_start (`KismetMathLibrary.RandomInteger` (`KismetArrayLibrary.Array_Length` _player_start))))
  ;[1 1 1] Spawn Player at a random spawnpoint
  (`/Engine/EditorBlueprintResources/StandardMacros.IsValid` _returnvalue
    (:`Is Valid`
      (`self.K2_DestroyActor` _returnvalue))
    (:`Is Not Valid`
      _))
  (while (stale _returnvalue_2)
    (bind (_outactors _returnvalue_2) (`KismetSystemLibrary.SphereOverlapActors` (`self.K2_GetActorLocation` _output) 500.0 (`|MakeArray` "ObjectTypeQuery3" :!type "EObjectTypeQuery Enum") "/Game/FirstPerson/Blueprints/BP_FirstPersonCharacter.BP_FirstPersonCharacter_C")))
  (bind _returnvalue_3 (`|SpawnActorFromClass` "/Game/FirstPerson/Blueprints/BP_FirstPersonCharacter.BP_FirstPersonCharacter_C" (`self.GetTransform` _output) "Undefined" "MultiplyWithRoot" null null))
  (`self.Possess` _returnvalue_3))

(event `Despawn`
  (bind _returnvalue (`self.K2_GetPawn`))
  ;[1 1 1] Despawns Player and creates an Empty pawn
  (`/Engine/EditorBlueprintResources/StandardMacros.IsValid` _returnvalue
    (:`Is Valid`
      (bind _asbp_first_person_character (cast `/Game/FirstPerson/Blueprints/BP_FirstPersonCharacter` _returnvalue))
      (`/Game/FirstPerson/Blueprints/BP_FirstPersonCharacter.Remove Widgets` _asbp_first_person_character)
      (`self.K2_DestroyActor` _returnvalue))
    (:`Is Not Valid`
      _))
  (bind _returnvalue_2 (`|SpawnActorFromClass` "/Game/Quake/Misc_BluePrints/BP_EmptyPawn.BP_EmptyPawn_C" (`self.GetTransform`) "Undefined" "MultiplyWithRoot" null null))
  (set `self.Spawned` false)
  (`self.Possess` _returnvalue_2))

(event `K++`
  ;[1 1 1] Increment Kills
  (bind _result (`/Engine/EditorBlueprintResources/StandardMacros.IncrementInt` (`self.Kills`))
    (:`  `
      (set `self.Kills` _result))))

(event `Key|Tab`
  (params (Key :type "Key Structure"))
  (bind _returnvalue (`self.K2_GetPawn`))
  ;[0.2926 0.8393 1] Show KD
  (:`Pressed`
    (bind _asbp_first_person_character (cast `/Game/FirstPerson/Blueprints/BP_FirstPersonCharacter` _returnvalue))
    (`/Game/FirstPerson/Blueprints/BP_FirstPersonCharacter.Call Widget Show KD` _asbp_first_person_character))
  (:`Released`
    (bind _asbp_first_person_character_2 (cast `/Game/FirstPerson/Blueprints/BP_FirstPersonCharacter` _returnvalue))
    (`/Game/FirstPerson/Blueprints/BP_FirstPersonCharacter.Call Widget Hide KD` _asbp_first_person_character_2)))

(event `D++`
  ;[1 1 1] Increment Deaths
  (bind _result (`/Engine/EditorBlueprintResources/StandardMacros.IncrementInt` (`self.Deaths`))
    (:`  `
      (set `self.Deaths` _result))))

(fn `UserConstructionScript`)